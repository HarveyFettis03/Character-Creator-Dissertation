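; A Simon Says floor button actor that lights up when stepped on.
; On BeginPlay it creates a dynamic material and colours it red, green, yellow or blue from its Colours value.
; An overlap passes that colour to CorrectOrIncorrect, which decides whether the button glows for half a second or only flashes briefly.
; The glow sets emissive colour to a boosted copy of the button colour, then resets it to black.
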(event `self.ReceiveBeginPlay`
  (bind _staticmeshcomponent (`self.StaticMeshComponent`))
  (bind _staticmeshcomponent_2 (`self.StaticMeshComponent`))
  (bind _staticmeshcomponent_3 (`self.StaticMeshComponent`))
  (bind _returnvalue (`KismetMaterialLibrary.CreateDynamicMaterialInstance` (`PrimitiveComponent.GetMaterial` _staticmeshcomponent 0)))
  (bind _output_get (set `self.My Material` _returnvalue))
  (`PrimitiveComponent.SetMaterial` _staticmeshcomponent 0 _output_get)
  (switch `/Game/Character_Creator/Simon_Says/Blueprints/SS_Colours` (`self.Colours`)
    (:`NewEnumerator0`
      (`MeshComponent.SetVectorParameterValueOnMaterials` _staticmeshcomponent_2 "Colour" (1.0 0.0 0.0)))
    (:`NewEnumerator1`
      (`MeshComponent.SetVectorParameterValueOnMaterials` _staticmeshcomponent_2 "Colour" (0.0 1.0 0.0)))
    (:`NewEnumerator2`
      (`MeshComponent.SetVectorParameterValueOnMaterials` _staticmeshcomponent_3 "Colour" (1.0 1.0 0.0)))
    (:`NewEnumerator3`
      (`MeshComponent.SetVectorParameterValueOnMaterials` _staticmeshcomponent_3 "Colour" (0.0 0.0 1.0)))))

(event `self.ReceiveActorBeginOverlap`
  (params (OtherActor :type "Actor Object Reference"))
  ;[1 1 1] Lights up when player steps on the buttons if the player steps on correct button
  (bind _correct (`/Game/Character_Creator/Simon_Says/Blueprints/TriggerBox__For_SS__Blueprint.PlayerStepsOn` (`self.Correct or incorrect`) (`self.Colours`)))
  (if _correct
    (`self.Light On`)
    (`KismetSystemLibrary.Delay` 0.5)
    (`self.Light Off`)
    (else
      (`self.Light On`)
      (`KismetSystemLibrary.Delay` 0.01)
      (`self.Light Off`))))

(fn `Light Off`
  (`MaterialInstanceDynamic.SetVectorParameterValue` (`self.My Material`) "Emissive Colour" (make `LinearColor` 0.0 0.0 0.0 1.0)))

(fn `Light On`
  (bind _my_material (`self.My Material`))
  (bind _returnvalue (`MaterialInstanceDynamic.K2_GetVectorParameterValue` _my_material "Colour"))
  (`MaterialInstanceDynamic.SetVectorParameterValue` _my_material "Emissive Colour" (* _returnvalue 100.0)))

(fn `UserConstructionScript`)