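; Trigger box that runs a Simon Says color memory game, revealing a key when solved.
; Entering randomizes the sequence, flashes all SS_BluePrint lights and starts a looping timer that lights Red, Green, Yellow or Blue per step.
; After four steps, or on leaving, the timer is cleared; playback completion also lifts the input lockout.
; PlayerStepsOn checks each color against the sequence, playing a success or error sound and returning the result.
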(event `Simon Says Tick`
  (bind _yellow (`self.Yellow`))
  (bind _green (`self.Green`))
  (bind _red (`self.Red`))
  (bind _blue (`self.Blue`))
  ;[1 1 1] Set up for sequcnce
  (switch `/Game/Character_Creator/Simon_Says/Blueprints/SS_Colours` (`|GetArrayItem` (`self.Simon Sequence`) (`self.Sequence Number`))
    (:`NewEnumerator0`
      (`/Game/Character_Creator/Simon_Says/Blueprints/SS_BluePrint.Light On` _red)
      (`KismetSystemLibrary.Delay` (`self.SS Light Duration`))
      (`/Game/Character_Creator/Simon_Says/Blueprints/SS_BluePrint.Light Off` _red))
    (:`NewEnumerator1`
      (`/Game/Character_Creator/Simon_Says/Blueprints/SS_BluePrint.Light On` _green)
      (`KismetSystemLibrary.Delay` (`self.SS Light Duration`))
      (`/Game/Character_Creator/Simon_Says/Blueprints/SS_BluePrint.Light Off` _green))
    (:`NewEnumerator2`
      (`/Game/Character_Creator/Simon_Says/Blueprints/SS_BluePrint.Light On` _yellow)
      (`KismetSystemLibrary.Delay` (`self.SS Light Duration`))
      (`/Game/Character_Creator/Simon_Says/Blueprints/SS_BluePrint.Light Off` _yellow))
    (:`NewEnumerator3`
      (`/Game/Character_Creator/Simon_Says/Blueprints/SS_BluePrint.Light On` _blue)
      (`KismetSystemLibrary.Delay` (`self.SS Light Duration`))
      (`/Game/Character_Creator/Simon_Says/Blueprints/SS_BluePrint.Light Off` _blue)))
  (`KismetSystemLibrary.Delay` (`self.Duration between one light on and other light on`))
  (bind _result (`/Engine/EditorBlueprintResources/StandardMacros.IncrementInt` (`self.Sequence Number`))
    (:`  `
      (if (>= _result 4)
        (set `self.LockOut` false)
        (set `self.Sequence Number` 0)
        ;[1 1 1] Crossing over the Trigger Box to start the game and makes a random sequence for the SS game
        (`KismetSystemLibrary.K2_ClearAndInvalidateTimerHandle` (stale `self.ReceiveActorBeginOverlap` _returnvalue) :!label _label)))))

(event `self.ReceiveActorBeginOverlap`
  (params (OtherActor :type "Actor Object Reference"))
  (bind _simon_sequence (`self.Simon Sequence`))
  ;[1 1 1] Crossing over the Trigger Box to start the game and makes a random sequence for the SS game
  (set `self.LockOut` true)
  (`KismetSystemLibrary.PrintString` "Simon Says Begin")
  (for (_ _array_index) _simon_sequence
    (`KismetArrayLibrary.Array_Set` _simon_sequence _array_index (`KismetArrayLibrary.Array_Random` (`self.Ran Colours`))))
  (set `self.Sequence Number` 0)
  (set `self.Answer Number` 0)
  (bind _returnvalue (`KismetSystemLibrary.K2_SetTimerDelegate` (delegate `Simon Says Tick`) 1.2 true))
  (bind _outactors (`GameplayStatics.GetAllActorsOfClass` "/Game/Character_Creator/Simon_Says/Blueprints/SS_BluePrint.SS_BluePrint_C"))
  (for _array_element _outactors
    (`/Game/Character_Creator/Simon_Says/Blueprints/SS_BluePrint.Light On` _array_element))
  (`KismetSystemLibrary.Delay` (`self.Duration between one light on and other light on`))
  (for _array_element_2 _outactors
    (`/Game/Character_Creator/Simon_Says/Blueprints/SS_BluePrint.Light Off` _array_element_2)))

(event `self.ReceiveActorEndOverlap`
  (params (OtherActor :type "Actor Object Reference"))
  ;[1 1 1] Crossing over the Trigger Box to start the game and makes a random sequence for the SS game
  (`KismetSystemLibrary.PrintString` "End of SS")
  (goto _label))

(fn `PlayerStepsOn`
  (params (Colour :type "/Game/Character_Creator/Simon_Says/Blueprints/SS_Colours Enum" :default "NewEnumerator0"))
  (returns (Correct :type Boolean))
  (if (`self.LockOut`)
    (return true)
    (elif (`|EnumEquality` Colour (`|GetArrayItem` (`self.Simon Sequence`) (`self.Answer Number`)))
      (bind _result (`/Engine/EditorBlueprintResources/StandardMacros.IncrementInt` (`self.Answer Number`))
        (:`  `
          (if (>= _result 4)
            (`GameplayStatics.PlaySound2D` "/Game/Character_Creator/Simon_Says/Sounds/131660__bertrof__game-sound-correct.131660__bertrof__game-sound-correct" 0.25 1.0 0.0 null null)
            (set `self.LockOut` true)
            (bind _returnvalue (`GameplayStatics.GetActorOfClass` "/Game/Character_Creator/Simon_Says/Blueprints/BP_SS_Key.BP_SS_Key_C"))
            (`SceneComponent.SetVisibility` (`/Game/Character_Creator/Simon_Says/Blueprints/BP_SS_Key.StaticMesh` _returnvalue) true false)
            (return true)
            (else
              (return true)))))
      (else
        (`GameplayStatics.PlaySound2D` "/Game/Character_Creator/Simon_Says/Sounds/700641__producing_raylite__incorrect-buzzer.700641__producing_raylite__incorrect-buzzer" 0.25 1.0 0.0 null null)
        (return false)))))

(fn `UserConstructionScript`)