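; BP_Dialogue is an interactable dialogue actor that shows lines of text and, once finished, reveals the BP_Key mesh in the level.
; A trigger zone toggles a widget component's visibility on overlap begin and end, without filtering the overlapping actor.
; Each Interact call advances the index through the Dialogue array, creating WB_Dialogue when none is valid and setting its text.
; Past the last line, it removes the box and makes the key visible.
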(event `/Game/Character_Creator/Level_Objects/BPI_Interact.Interact`
  (`/Engine/EditorBlueprintResources/StandardMacros.IncrementInt` (`self.Dialogue Index`)
    (:`  `
      (if (< (`self.Dialogue Index`) (`KismetArrayLibrary.Array_Length` (`self.Dialogue`)))
        (`self.DialogueBox`
          (:`then`
            _)
          (:`else`
            (bind _returnvalue (`|CreateWidget` "/Game/Character_Creator/Dialogue/WB_Dialogue.WB_Dialogue_C" (`GameplayStatics.GetPlayerController` 0)))
            (bind _output_get (set `self.DialogueBox` _returnvalue))
            (`UserWidget.AddToViewport` _output_get 0)))
        (`TextBlock.SetText` (`/Game/Character_Creator/Dialogue/WB_Dialogue.DialogueText` (`self.DialogueBox`)) (`KismetTextLibrary.Conv_StringToText` (`|GetArrayItem` (`self.Dialogue`) (`self.Dialogue Index`))))
        (else
          (`Widget.RemoveFromParent` (`self.DialogueBox`))
          (bind _returnvalue_2 (`GameplayStatics.GetActorOfClass` "/Game/Character_Creator/Level_Objects/BP_Key.BP_Key_C"))
          (`SceneComponent.SetVisibility` (`/Game/Character_Creator/Level_Objects/BP_Key.StaticMesh` _returnvalue_2) true false))))))

(event `self.Trigger Zone.OnComponentBeginOverlap`
  (params (OverlappedComponent :type "PrimitiveComponent Object Reference") (OtherActor :type "Actor Object Reference") (OtherComp :type "PrimitiveComponent Object Reference") (OtherBodyIndex :type Integer) (bFromSweep :type Boolean) (SweepResult :type "HitResult Structure (by ref)"))
  (`SceneComponent.SetVisibility` (`self.Widget`) true false))

(event `self.Trigger Zone.OnComponentEndOverlap`
  (params (OverlappedComponent :type "PrimitiveComponent Object Reference") (OtherActor :type "Actor Object Reference") (OtherComp :type "PrimitiveComponent Object Reference") (OtherBodyIndex :type Integer))
  (`SceneComponent.SetVisibility` (`self.Widget`) false false))

(fn `UserConstructionScript`)